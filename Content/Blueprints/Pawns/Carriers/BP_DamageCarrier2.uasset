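; BP_DamageCarrier2 is a damageable carrier Blueprint that shows its health on a world-space bar facing the player's camera.
; On BeginPlay it caches the WBP_EnemyHealth widget, fills the bar and binds to the HealthComponent's health-set event.
; Health changes set the bar's percent relative to MaxHP.
; A looping timer, rather than Tick, drives the billboard rotation toward the camera.
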(event Custom|Rotate%20HP%20Widget
  (Transformation|SetWorldRotation (Variables|Default|GetHP%20Widget) (Math|Rotator|FindLookatRotation (Transformation|GetWorldLocation (Variables|Default|GetHP%20Widget)) (Transformation|GetWorldLocation (Variables|/Script/Engine.PlayerCameraManager|GetTransformComponent (Game|GetPlayerCameraManager 0)))) false false))

(event Custom|Update%20HP%20Widget
  (params (NewHealth :type Float%20%28single-precision%29))
  (CallFunction|SetNewHP NewHealth))

(event EventBeginPlay
  (Utilities|FlowControl|Sequence
    (:then_0
      (bind _aswbp_enemy_health (Utilities|Casting|CastToWBP_EnemyHealth (UserInterface|GetWidget (Variables|Default|GetHP%20Widget))))
      (Variables|Default|SetEnemy%20Health _aswbp_enemy_health))
    (:then_1
      (Utilities|Time|SetTimerbyEvent (EventDispatchers|CreateEvent :!event Custom|Rotate%20HP%20Widget) 0.1 true true))
    (:then_2
      (CallFunction|SetNewHP (Variables|/Script/SpaceWar.HealthComponent|GetMaxHP (Variables|Default|GetHealthComponent))))
    (:then_3
      (EventDispatchers|BindEventtoOnSetHealth (Variables|Default|GetHealthComponent) (EventDispatchers|CreateEvent :!event Custom|Update%20HP%20Widget)))))

(fn ConstructionScript)

(fn SetNewHP
  (params (New%20Health :type Float%20%28double-precision%29))
  (Progress|SetPercent (Variables|/Game/Blueprints/Widgets/HP/WBP_EnemyHealth.WBP_EnemyHealth_C|GetHealthBar (Variables|Default|GetEnemy%20Health)) (/ New%20Health (Variables|/Script/SpaceWar.HealthComponent|GetMaxHP (Variables|Default|GetHealthComponent)))))