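; Player pawn Blueprint for a craft with engine beams and trails, acting mainly as the HUD layer for health, weapons and aiming.
; BeginPlay creates the health, weapons and twin crosshair widgets and starts looping timers for frequent updates.
; Event handlers refresh HP, swap crosshair texture and ammo binding per gun, and toggle a rocket-lock warning.
; Death deactivates the effects, then opens the start menu after a delay.
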(event OnSetHealth(RegeneratableHealth)
  (params (NewHealth :type Float%20%28single-precision%29))
  (CallFunction|SetHP NewHealth))

(event Custom|OnRocketFollowAdded_Event
  (if (Utilities|IsValid (Variables|Default|GetAttentionWidget))
    (Widget|SetVisibility (Variables|Default|GetAttentionWidget) "Visible")
    (else
      (bind _returnvalue (UserInterface|CreateWidget "/Game/Blueprints/Widgets/EnemyRockets/WBP_RocketWarning.WBP_RocketWarning_C"))
      (bind _output_get (Variables|Default|SetAttentionWidget _returnvalue))
      (UserInterface|Viewport|AddtoViewport _output_get 0)
      (Widget|SetVisibility (Variables|Default|GetAttentionWidget) "Visible"))))

(event Custom|OnRocketFollowRemoved_Event
  (if (Utilities|IsValid (Variables|Default|GetAttentionWidget))
    (bind _returnvalue (Class|SpaceShipBase|RocketsFollowedCount))
    (if (== _returnvalue 0)
      (Widget|SetVisibility (Variables|Default|GetAttentionWidget) "Hidden"))))

(event Custom|CreateCrosshair
  (bind _returnvalue (UserInterface|CreateWidget "/Game/Blueprints/Widgets/Crosshair/WBP_Crosshair.WBP_Crosshair_C"))
  (bind _output_get (Variables|Default|SetCrosshair01 _returnvalue))
  (UserInterface|Viewport|AddtoViewport _output_get 0)
  (bind _returnvalue_2 (UserInterface|CreateWidget "/Game/Blueprints/Widgets/Crosshair/WBP_Crosshair.WBP_Crosshair_C"))
  (bind _output_get_2 (Variables|Default|SetCrosshair02 _returnvalue_2))
  (UserInterface|Viewport|AddtoViewport _output_get_2 0))

(event Custom|SetAbilitiesCooldowns
  (Default|SetCooldowns (Variables|Default|GetWeapons)))

(event Custom|OnDeath_Event
  (Components|Activation|Deactivate (Variables|Default|GetRightTrail))
  (Components|Activation|Deactivate (Variables|Default|GetEngineBeam2))
  (Components|Activation|Deactivate (Variables|Default|GetEngineBeam1))
  (Components|Activation|Deactivate (Variables|Default|GetLeftTrail))
  (Utilities|FlowControl|Delay 4.0)
  (Game|OpenLevel(byObjectReference) "/Game/Maps/L_StartMenu.L_StartMenu"))

(event Custom|ChangeCrosshair
  (params (NewGun :type Gun%20Scene%20Component%20Object%20Reference) (PreviouseGun :type Gun%20Scene%20Component%20Object%20Reference))
  (if (Utilities|IsValid PreviouseGun)
    (EventDispatchers|UnbindEventfromOnBulletCountChanged PreviouseGun (EventDispatchers|CreateEvent :!event SetNewAmmoCount)))
  (CallFunction|SetNewCrosshairImage NewGun)
  (bind _returnvalue (Class|GunSceneComponent|GetAmmo NewGun))
  (Default|SetAmmo (Variables|Default|GetWeapons) _returnvalue)
  (EventDispatchers|BindEventtoOnBulletCountChanged NewGun (EventDispatchers|CreateEvent :!event SetNewAmmoCount)))

(event Custom|OnItemAdded_Event
  (params (Value :type Item%20Data%20Asset%20Object%20Reference)))

(event EventBeginPlay
  (bind _returnvalue (UserInterface|CreateWidget "/Game/Blueprints/Widgets/HP/WBP_PlayerHealth.WBP_PlayerHealth_C"))
  (bind _output_get (Variables|Default|SetHealth%20Widget _returnvalue))
  (UserInterface|Viewport|AddtoViewport _output_get 0)
  (CallFunction|CreateCrosshair)
  (Utilities|Time|SetTimerbyEvent (EventDispatchers|CreateEvent :!event MoveCrosshair) 0.01 true true)
  (CallFunction|SetHP (Variables|/Script/SpaceWar.HealthComponent|GetCurrentHP (Variables|Default|GetRegeneratableHealth)))
  (bind _returnvalue_2 (UserInterface|CreateWidget "/Game/Blueprints/Widgets/Weapons/WBP_Weapons.WBP_Weapons_C"))
  (bind _output_get_2 (Variables|Default|SetWeapons _returnvalue_2))
  (UserInterface|Viewport|AddtoViewport _output_get_2 0)
  (EventDispatchers|BindEventtoOnEquipped (EventDispatchers|CreateEvent :!event Custom|ChangeCrosshair))
  (EventDispatchers|BindEventtoOnRocketFollowAdded (EventDispatchers|CreateEvent :!event Custom|OnRocketFollowAdded_Event))
  (EventDispatchers|BindEventtoOnRocketFollowRemoved (EventDispatchers|CreateEvent :!event Custom|OnRocketFollowRemoved_Event))
  (Utilities|Time|SetTimerbyEvent (EventDispatchers|CreateEvent :!event Custom|SetAbilitiesCooldowns) 0.02 true true)
  (EventDispatchers|BindEventtoOnDeath (EventDispatchers|CreateEvent :!event Custom|OnDeath_Event)))

(event Collision|EventActorBeginOverlap
  (params (OtherActor :type Actor%20Object%20Reference)))

(event EventTick
  (params (DeltaSeconds :type Float%20%28single-precision%29)))

(fn ConstructionScript)

(fn MoveCrosshair
  (bind _returnvalue (Class|PlayerShip|GetPlayerAimDirection01))
  (Default|SetCrosshairPosition (Variables|Default|GetCrosshair01) _returnvalue)
  (bind _returnvalue_2 (Class|PlayerShip|GetPlayerAimDirection02))
  (Default|SetCrosshairPosition (Variables|Default|GetCrosshair02) _returnvalue_2))

(fn SetHP
  (params (A :type Float%20%28double-precision%29))
  (bind _health_widget (Variables|Default|GetHealth%20Widget))
  (if (Utilities|IsValid _health_widget)
    (Default|SetHP _health_widget A (Variables|/Script/SpaceWar.HealthComponent|GetMaxHP (Variables|Default|GetRegeneratableHealth)))))

(fn SetNewCrosshairImage
  (params (Weapon :type Gun%20Scene%20Component%20Object%20Reference))
  (bind _crosshairtexture (Variables|/Script/SpaceWar.GunSceneComponent|GetCrosshairTexture Weapon))
  (Default|SetCrosshair (Variables|Default|GetCrosshair01) _crosshairtexture)
  (Default|SetCrosshair (Variables|Default|GetCrosshair02) _crosshairtexture))

(fn SetNewAmmoCount
  (params (NewAmmoValue :type Integer))
  (Default|SetAmmo (Variables|Default|GetWeapons) NewAmmoValue))