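; Boss helicopter Blueprint that shows an on-screen health bar for the boss.
; On BeginPlay it creates a WBP_BossHealth widget, adds it to the viewport, sets the boss name and fills it to the HealthComponent's max HP.
; It binds to the component's OnSetHealth event, so the widget follows health changes without polling on Tick.
; The graph holds no movement or attack logic.
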(event Custom|OnSetHealth_Event
  (params (NewHealth :type Float%20%28single-precision%29))
  (Default|SetHealth (Variables|Default|GetBossHPWidget) NewHealth (Variables|/Script/SpaceWar.HealthComponent|GetMaxHP (Variables|Default|GetHealthComponent))))

(event EventBeginPlay
  (bind _healthcomponent (Variables|Default|GetHealthComponent))
  (bind _maxhp (Variables|/Script/SpaceWar.HealthComponent|GetMaxHP _healthcomponent))
  (bind _returnvalue (UserInterface|CreateWidget "/Game/Blueprints/Widgets/HP/WBP_BossHealth.WBP_BossHealth_C"))
  (UserInterface|Viewport|AddtoViewport _returnvalue 0)
  (bind _output_get (Variables|Default|SetBossHPWidget _returnvalue))
  (Default|SetName _output_get (Variables|Default|GetBossName))
  (EventDispatchers|AssignOnSetHealth (Variables|Default|GetHealthComponent) (delegate Custom|OnSetHealth_Event))
  (Default|SetHealth (Variables|Default|GetBossHPWidget) _maxhp _maxhp))

(event Collision|EventActorBeginOverlap
  (params (OtherActor :type Actor%20Object%20Reference)))

(event EventTick
  (params (DeltaSeconds :type Float%20%28single-precision%29)))

(fn ConstructionScript)