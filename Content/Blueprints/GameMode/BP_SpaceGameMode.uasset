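; Space shooter game mode that manages HUD widgets, level music and the boss-to-next-level transition.
; BeginPlay caches the PlayerShip, creates effects and timer widgets, and binds upgrade, timer and task-completion delegates.
; Events update ammo, dual aim-driven crosshairs, rocket warnings and difficulty popups; the HP setter is an empty stub.
; Spawning the boss switches the music, and its death leads to loading NextLevel after a short delay.
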(event Custom|Move%20Crosshair
  ;[1 1 1] Move crosshair event
  (bind _returnvalue (Class|PlayerShip|GetPlayerAimDirection01 (Variables|Default|GetCharacterReference)))
  (Default|SetCrosshairPosition (Variables|Default|GetCrosshair02) _returnvalue)
  (bind _returnvalue_2 (Class|PlayerShip|GetPlayerAimDirection02 (Variables|Default|GetCharacterReference)))
  (Default|SetCrosshairPosition (Variables|Default|GetCrosshair01) _returnvalue_2))

(event Custom|SetNewAmmoCount
  (params (Ammo :type Integer))
  ;[1 1 1] Set new ammo count in widget
  (Default|SetAmmo (Variables|Default|GetWeapons) Ammo))

(event Custom|BossKilled
  (Utilities|FlowControl|Delay 2.0)
  (CallFunction|LoadNextLvl))

(event Custom|StartBossMusic
  (Audio|Components|Audio|SetSound (Variables|Default|GetAudio) (Variables|Default|GetBossMusic))
  (Audio|Components|Audio|Play (Variables|Default|GetAudio) 0.0))

(event Custom|StartMusic
  (Audio|Components|Audio|SetSound (Variables|Default|GetAudio) (Variables|Default|GetLevelMusic))
  (Audio|Components|Audio|Play (Variables|Default|GetAudio) 0.0))

(event Custom|SpawnLevelBoss
  (bind _returnvalue (Class|SpaceGameMode|SpawnBoss))
  (EventDispatchers|BindEventtoOnDestroy _returnvalue (EventDispatchers|CreateEvent :!event Custom|BossKilled))
  (CallFunction|StartBossMusic))

(event Custom|Set%20HP
  (params (NewHealth :type Float%20%28single-precision%29))
  ;[1 1 1] Set player HP in widget
  (CallFunction|SetHPPercent NewHealth))

(event Custom|HideRocketWarning
  ;[1 1 1] Hide following rocket warning widget
  (if (Utilities|IsValid (Variables|Default|GetAttentionWidget))
    (bind _returnvalue (Class|SpaceShipBase|RocketsFollowedCount (Variables|Default|GetCharacterReference)))
    (if (== _returnvalue 0)
      (Widget|SetVisibility (Variables|Default|GetAttentionWidget) "Hidden"))))

(event Custom|ShowRocketWarning
  ;[1 1 1] Show following rocket warning widget
  (if (Utilities|IsValid (Variables|Default|GetAttentionWidget))
    (Widget|SetVisibility (Variables|Default|GetAttentionWidget) "Visible")
    (else
      (bind _returnvalue (UserInterface|CreateWidget "/Game/Blueprints/Widgets/EnemyRockets/WBP_RocketWarning.WBP_RocketWarning_C"))
      (bind _output_get (Variables|Default|SetAttentionWidget _returnvalue))
      (UserInterface|Viewport|AddtoViewport _output_get 0)
      (Widget|SetVisibility (Variables|Default|GetAttentionWidget) "Visible"))))

(event Custom|OnDifficultyChanged
  (params (value :type Integer))
  ;[1 1 1] Difficulty changed widget
  (bind _returnvalue (UserInterface|CreateWidget "/Game/Blueprints/Widgets/Misc/WBP_DifficultyChanged.WBP_DifficultyChanged_C"))
  (Default|SetLevel _returnvalue value)
  (UserInterface|Viewport|AddtoViewport _returnvalue 0)
  (Utilities|FlowControl|Delay 2.0)
  (Widget|RemovefromParent _returnvalue))

(event Custom|ChangeCrosshair
  (params (NewGun :type Gun%20Scene%20Component%20Object%20Reference) (PreviouseGun :type Gun%20Scene%20Component%20Object%20Reference))
  ;[1 1 1] Change crosshair image event
  (if (Utilities|IsValid PreviouseGun)
    (EventDispatchers|UnbindEventfromOnBulletCountChanged PreviouseGun (EventDispatchers|CreateEvent :!event Custom|SetNewAmmoCount)))
  (CallFunction|SetNewCrosshairImage NewGun)
  (bind _returnvalue (Class|GunSceneComponent|GetAmmo NewGun))
  (Default|SetAmmo (Variables|Default|GetWeapons) _returnvalue)
  (EventDispatchers|BindEventtoOnBulletCountChanged NewGun (EventDispatchers|CreateEvent :!event Custom|SetNewAmmoCount)))

(event Custom|DisplayAllTasks
  (Development|PrintString (Utilities|String|ToString(Integer) (Utilities|Array|Length (Variables|Default|GetTasks)))))

(event Custom|SetTime
  (bind _gameinstance (Variables|Default|GetGameInstance))
  ;[1 1 1] World Timer
  (Default|SetTime (Variables|Default|GetTimerWidget) (Class|SpaceGameInstance|GetMinutes _gameinstance) (Class|SpaceGameInstance|GetSeconds _gameinstance)))

(event Custom|LoadNextLvl
  (Game|OpenLevel(byObjectReference) (Variables|Default|GetNextLevel) false))

(event EventBeginPlay
  (bind _returnvalue (Game|GetPlayerController 0))
  (CallFunction|GetPlayerReference)
  (CallFunction|CreateEffectsWidget)
  (EventDispatchers|BindEventtoOnUpgraded (Variables|Default|GetGameInstance) (EventDispatchers|CreateEvent :!event Custom|OnDifficultyChanged))
  (CallFunction|CreateTimerWidget)
  (EventDispatchers|BindEventtoOnTimerChanged (Variables|Default|GetGameInstance) (EventDispatchers|CreateEvent :!event Custom|SetTime))
  (EventDispatchers|BindEventtoOnAllTasksCompleted (EventDispatchers|CreateEvent :!event Custom|SpawnLevelBoss))
  (Input|SetInputModeGameOnly _returnvalue false)
  (Variables|/Script/Engine.PlayerController|SetbShowMouseCursor _returnvalue false)
  (CallFunction|StartMusic))

(fn ConstructionScript)

(fn StartMovementCrosshairWidget
  (Utilities|Time|SetTimerbyEvent (EventDispatchers|CreateEvent :!event Custom|Move%20Crosshair) 0.01 true true))

(fn CreateCrosshairWidget
  (bind _returnvalue (UserInterface|CreateWidget "/Game/Blueprints/Widgets/Crosshair/WBP_Crosshair.WBP_Crosshair_C"))
  (bind _output_get (Variables|Default|SetCrosshair02 _returnvalue))
  (UserInterface|Viewport|AddtoViewport _output_get 0)
  (bind _returnvalue_2 (UserInterface|CreateWidget "/Game/Blueprints/Widgets/Crosshair/WBP_Crosshair.WBP_Crosshair_C"))
  (bind _output_get_2 (Variables|Default|SetCrosshair01 _returnvalue_2))
  (UserInterface|Viewport|AddtoViewport _output_get_2 0))

(fn CreateHPWidget
  (bind _returnvalue (UserInterface|CreateWidget "/Game/Blueprints/Widgets/HP/WBP_PlayerHealth.WBP_PlayerHealth_C"))
  (bind _output_get (Variables|Default|SetHealthWidget _returnvalue))
  (UserInterface|Viewport|AddtoViewport _output_get 0))

(fn GetPlayerReference
  (bind _asplayer_ship (Utilities|Casting|CastToPlayerShip (Game|Player|GetPlayerPawn 0)))
  (bind _output_get (Variables|Default|SetCharacterReference _asplayer_ship))
  (Development|PrintString (Utilities|GetDisplayName _output_get)))

(fn BindHPChangeDelegate)

(fn SetHPPercent
  (params (HP :type Float%20%28double-precision%29)))

(fn CreateEffectsWidget
  (bind _returnvalue (UserInterface|CreateWidget "/Game/Blueprints/Widgets/Effects/WBP_Effects.WBP_Effects_C"))
  (bind _output_get (Variables|Default|SetEffectsWidget _returnvalue))
  (UserInterface|Viewport|AddtoViewport _output_get 0))

(fn CreateWeaponsWidget
  (bind _returnvalue (UserInterface|CreateWidget "/Game/Blueprints/Widgets/Weapons/WBP_Weapons.WBP_Weapons_C"))
  (bind _output_get (Variables|Default|SetWeapons _returnvalue))
  (UserInterface|Viewport|AddtoViewport _output_get 0))

(fn SetNewCrosshairImage
  (params (Weapon :type Gun%20Scene%20Component%20Object%20Reference))
  (bind _crosshairtexture (Variables|/Script/SpaceWar.GunSceneComponent|GetCrosshairTexture Weapon))
  (Default|SetCrosshair (Variables|Default|GetCrosshair01) _crosshairtexture)
  (Default|SetCrosshair (Variables|Default|GetCrosshair02) _crosshairtexture))

(fn CreateTimerWidget
  (bind _returnvalue (UserInterface|CreateWidget "/Game/Blueprints/Widgets/Misc/WBP_WorldTimer.WBP_WorldTimer_C"))
  (bind _output_get (Variables|Default|SetTimerWidget _returnvalue))
  (CallFunction|SetTime)
  (UserInterface|Viewport|AddtoViewport _output_get 0))

(fn GetRandomFloat
  (params (Min :type Float%20%28double-precision%29) (Max :type Float%20%28double-precision%29) (CanBeLessZero :type Boolean)))