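; BP_MenuGameMode is the game mode for a menu, setting up its interface and music when play begins.
; On BeginPlay it creates the menu widget, adds it to the viewport, and switches the first player controller to UI-only input with a visible cursor.
; It then assigns the music sound to its audio component and plays it; Tick and the construction script are empty.
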(event EventBeginPlay
  (bind _returnvalue (Game|GetPlayerController 0))
  (bind _returnvalue_2 (UserInterface|CreateWidget (Variables|Default|GetMenuWidget)))
  (UserInterface|Viewport|AddtoViewport _returnvalue_2 0)
  (Input|SetInputModeUIOnly _returnvalue 0 "DoNotLock" false)
  (Variables|/Script/Engine.PlayerController|SetbShowMouseCursor _returnvalue true)
  (Audio|Components|Audio|SetSound (Variables|Default|GetAudio) (Variables|Default|GetMusic))
  (Audio|Components|Audio|Play (Variables|Default|GetAudio) 0.0))

(event EventTick
  (params (DeltaSeconds :type Float%20%28single-precision%29)))

(fn ConstructionScript)