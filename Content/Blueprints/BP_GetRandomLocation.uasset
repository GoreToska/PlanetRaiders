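; Behavior tree task that picks a random patrol position and writes it to a Blackboard vector key.
; Each axis is randomized within plus or minus PatrolRadius around the world origin, as the controlled pawn's location is unused.
; A box overlap test at that point sets the result: success when no actors overlap, failure otherwise, with the key written either way.
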(event EventReceiveExecuteAI
  (params (OwnerController :type AI%20Controller%20Object%20Reference) (ControlledPawn :type Pawn%20Object%20Reference))
  (bind _patrolradius (Variables|Default|GetPatrolRadius))
  (bind _patrolradius_2 (Variables|Default|GetPatrolRadius))
  (bind _patrolradius_3 (Variables|Default|GetPatrolRadius))
  (bind _output_get (Variables|Default|SetRandomPosition (Math|Vector|MakeVector (Math|Random|RandomFloatinRange (- 0.0 _patrolradius_2) _patrolradius_2) (Math|Random|RandomFloatinRange (- 0.0 _patrolradius_3) _patrolradius_3) (Math|Random|RandomFloatinRange (- 0.0 _patrolradius) _patrolradius))))
  (bind _returnvalue (Collision|BoxOverlapActors _output_get "100.000000,100.000000,100.000000" (Variables|Default|GetObject%20Types) "/Script/Engine.Actor" :!class /Script/Engine.KismetSystemLibrary))
  (AI|BehaviorTree|SetBlackboardValueasVector (Variables|Default|GetKey) _output_get)
  (AI|BehaviorTree|FinishExecute (not _returnvalue)))