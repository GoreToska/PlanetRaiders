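; BP_Indicator is an actor that displays an on-screen marker for its world location, pinned to the screen edge when off-screen.
; On BeginPlay it creates a WBP_IndicatorBase widget with its color and text.
; A looping timer repositions it via FindScreenEdgeLocationForWorldLocation, showing text when on-screen and a rotated off-screen texture without text otherwise.
; The widget follows visibility-change events and is removed when the actor is destroyed.
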(event Custom|Visibility
  (params (value :type Boolean))
  (bind _widget (Variables|Default|GetWidget))
  (if value
    (Widget|SetVisibility _widget "Visible")
    (else
      (Widget|SetVisibility _widget "Collapsed"))))

(event Custom|OnDestroyed_Event
  (params (DestroyedActor :type Actor%20Object%20Reference))
  (Widget|RemovefromParent (Variables|Default|GetWidget)))

(event Custom|Indicator
  (bind _returnvalue (Transformation|GetActorLocation))
  (bind _widget (Variables|Default|GetWidget))
  (bind _widget_2 (Variables|Default|GetWidget))
  (bind _edgepercent (Variables|Default|GetEdgePercent))
  (bind (_outscreenposition _outrotationangledegrees _bisonscreen) (Class|OffscreenIndicator|FindScreenEdgeLocationforWorldLocation _returnvalue _edgepercent))
  (bind _image (Variables|/Game/Blueprints/Widgets/Indicators/WBP_IndicatorBase.WBP_IndicatorBase_C|GetImage _widget))
  (bind _image_2 (Variables|/Game/Blueprints/Widgets/Indicators/WBP_IndicatorBase.WBP_IndicatorBase_C|GetImage _widget_2))
  (if _bisonscreen
    (Class|UserWidget|SetPositioninViewport (Variables|Default|GetWidget) _outscreenposition true)
    (Utilities|FlowControl|Sequence
      (:then_0
        (if (not (== (Class|Widget|GetRenderTransformAngle _image_2) 0.0))
          (Class|Widget|SetRenderTransformAngle _image_2 0.0)))
      (:then_1
        (if (not (== (Variables|/Game/Blueprints/Widgets/Indicators/WBP_IndicatorBase.WBP_IndicatorBase_C|GetImage (Variables|Default|GetWidget)) (Variables|Default|GetOffScreenTexture)))
          (Default|SetImage (Variables|Default|GetWidget) (Variables|Default|GetInScreenTexture))
          (Default|SetTextVisibility (Variables|Default|GetWidget) true))))
    (else
      (Class|UserWidget|SetPositioninViewport (Variables|Default|GetWidget) _outscreenposition true)
      (Class|Widget|SetRenderTransformAngle _image _outrotationangledegrees)
      (if (not (== _image (Variables|Default|GetOffScreenTexture)))
        (Default|SetImage (Variables|Default|GetWidget) (Variables|Default|GetOffScreenTexture))
        (Default|SetTextVisibility (Variables|Default|GetWidget) false)))))

(event EventBeginPlay
  (bind _returnvalue (UserInterface|CreateWidget "/Game/Blueprints/Widgets/Indicators/WBP_IndicatorBase.WBP_IndicatorBase_C"))
  (bind _output_get (Variables|Default|SetWidget _returnvalue))
  (Default|SetColor _output_get (Variables|Default|GetColor))
  (Default|SetTextValue _output_get (Variables|Default|GetText))
  (UserInterface|Viewport|AddtoViewport _output_get 0)
  (Class|UserWidget|SetPositioninViewport (Variables|Default|GetWidget) (Math|Conversions|ToVector2D(Vector) (Transformation|GetActorLocation)) true)
  (Utilities|Time|SetTimerbyEvent (delegate Custom|Indicator) 0.01 true true)
  (EventDispatchers|BindEventtoOnDestroyed (delegate Custom|OnDestroyed_Event))
  (EventDispatchers|BindEventtoOnVisibilityChanged (delegate Custom|Visibility)))

(event EventDestroyed
  (Widget|RemovefromParent (Variables|Default|GetWidget)))

(fn ConstructionScript)